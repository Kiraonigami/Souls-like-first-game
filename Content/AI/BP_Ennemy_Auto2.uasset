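; Enemy AI character Blueprint with a sword attack and a stats component whose health bar is set on BeginPlay.
; SwordAttack plays a combo montage, while Begin and End sword trace events start and clear a looping timer.
; Each timer tick sphere-traces for pawns between two points on the sword and applies damage, using a resettable DoOnce with a short delay to limit repeat hits.
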(event `self.ReceiveBeginPlay`
  (`/Game/Blueprints/BPC_Stats.Set Health Progress Bar` (`self.BPC_Stats`) null))

(event `/Game/Blueprints/BPI_Damage.EndSwordTrace`
  ;[0.2573 0.2573 0.2573] Sword Traces
  (if (`KismetSystemLibrary.K2_IsValidTimerHandle` (stale `/Game/Blueprints/BPI_Damage.BeginSwordTrace` _returnvalue))
    (`KismetSystemLibrary.K2_ClearAndInvalidateTimerHandle` (stale `/Game/Blueprints/BPI_Damage.BeginSwordTrace` _returnvalue))))

(event `/Game/Blueprints/BPI_Damage.BeginSwordTrace`
  ;[0.2573 0.2573 0.2573] Sword Traces
  (bind _returnvalue (`KismetSystemLibrary.K2_SetTimerDelegate` (delegate `Damage Trace`) 0.1 true)))

(event `Damage Trace`
  ;[0.2573 0.2573 0.2573] Sword Traces
  (bind (_outhit _returnvalue) (`KismetSystemLibrary.SphereTraceSingleForObjects` :`Start` (`SceneComponent.K2_GetComponentLocation` (`self.Start Sword Trace Pos`)) :`End` (`SceneComponent.K2_GetComponentLocation` (`self.End Sword Trace Pos`)) :`Radius` 25.0 :`ObjectTypes` (`|MakeArray` "ObjectTypeQuery3" :!type "EObjectTypeQuery Enum") :`DrawDebugType` "ForOneFrame"))
  (if _returnvalue
    (`/Engine/EditorBlueprintResources/StandardMacros.DoOnce` false :!label _label
      (:`Completed`
        (`GameplayStatics.ApplyDamage` (`.HitActor` (`GameplayStatics.BreakHitResult` _outhit)) (`self.Sword Damage`))
        (`KismetSystemLibrary.Delay` 0.3)
        (goto _label :!via `Reset`)))))

(fn `Sword Attack`
  (returns (Duration :type "Float (double-precision)"))
  (bind _returnvalue (`self.PlayAnimMontage` "/Game/Characters/Souls/Combat/SwordAttackCombo_Montage.SwordAttackCombo_Montage"))
  (return _returnvalue))

(fn `UserConstructionScript`)