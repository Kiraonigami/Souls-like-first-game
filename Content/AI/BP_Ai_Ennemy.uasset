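; BP_Ai_Ennemy is an enemy AI controller that runs a behavior tree from BeginPlay.
; Its PawnSensing component writes any seen pawn to the blackboard as the target actor and sets the seeing-target flag, which this graph never clears.
; The Big Attack and Sword Attack functions are empty stubs with no attack logic.
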(event `self.ReceiveBeginPlay`
  (`self.RunBehaviorTree` (`self.Behavior Tree`)))

(event `self.PawnSensing.OnSeePawn`
  (params (Pawn :type "Pawn Object Reference"))
  (`BlackboardComponent.SetValueAsBool` (`AIBlueprintHelperLibrary.GetBlackboard` null) "Seeing Target?" true)
  (`BlackboardComponent.SetValueAsObject` (`AIBlueprintHelperLibrary.GetBlackboard` null) "Target Actor" Pawn))

(fn `Big Attack`
  (returns (Duration :type "Float (double-precision)"))
  (return 0.0))

(fn `Sword Attack`
  (returns (Duration :type "Float (double-precision)")))

(fn `UserConstructionScript`)