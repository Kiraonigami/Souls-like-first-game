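; BP_Ennemy is a melee AI enemy character with a health bar widget driven by BPCStats, which also receives incoming damage.
; Montage attack functions play sound; a looping timer runs sword sphere traces between component or boss-specific points, with a DoOnce cooldown limiting hits.
; A separate point trace deals fixed damage and a delayed camera shake.
; Death disables movement, ragdolls the mesh and stops sword damage.
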(event `self.ReceiveBeginPlay`
  (bind _aswb_ennemy_health (cast `/Game/UI/WB_Ennemy_Health` (`WidgetComponent.GetWidget` (`self.Widget`))))
  (`/Game/Blueprints/BPC_Stats.Set Health Progress Bar` (`self.BPC_Stats`) (`/Game/UI/WB_Ennemy_Health.Healthbar` _aswb_ennemy_health)))

(event `self.ReceiveAnyDamage`
  (params (Damage :type "Float (single-precision)") (DamageType :type "DamageType Object Reference") (InstigatedBy :type "Controller Object Reference") (DamageCauser :type "Actor Object Reference"))
  (`/Game/Blueprints/BPC_Stats.Increase Value` (`self.BPC_Stats`) "NewEnumerator0" (* Damage -1.0)))

(event `/Game/Blueprints/BPI_Damage.EndSwordTrace`
  ;[0.2573 0.2573 0.2573] Sword Traces
  (if (`KismetSystemLibrary.K2_IsValidTimerHandle` (stale `/Game/Blueprints/BPI_Damage.BeginSwordTrace` _returnvalue))
    (`KismetSystemLibrary.K2_ClearAndInvalidateTimerHandle` (stale `/Game/Blueprints/BPI_Damage.BeginSwordTrace` _returnvalue))))

(event `/Game/Blueprints/BPI_Damage.BeginSwordTrace`
  ;[0.2573 0.2573 0.2573] Sword Traces
  (bind _returnvalue (`KismetSystemLibrary.K2_SetTimerDelegate` (delegate `Damage Trace`) 0.1 true)))

(event `Damage Trace`
  ;[0.2573 0.2573 0.2573] Sword Traces
  (if (not (`self.IsDead?`))
    (bind (_outhit _returnvalue) (`KismetSystemLibrary.SphereTraceSingleForObjects` :`Start` (`KismetMathLibrary.SelectVector` (`self.Boss Start Sword Trace `) (`SceneComponent.K2_GetComponentLocation` (`self.Start Sword Trace Pos`)) (`self.IsBoss?`)) :`End` (`KismetMathLibrary.SelectVector` (`self.Boss End Sword Trace`) (`SceneComponent.K2_GetComponentLocation` (`self.End Sword Trace Pos`)) (`self.IsBoss?`)) :`Radius` (`self.Sword Attack Radius`) :`ObjectTypes` (`|MakeArray` "ObjectTypeQuery3" :!type "EObjectTypeQuery Enum") :`DrawDebugType` "ForOneFrame"))
    (if _returnvalue
      (`/Engine/EditorBlueprintResources/StandardMacros.DoOnce` false :!label _label
        (:`Completed`
          (`GameplayStatics.ApplyDamage` (`.HitActor` (`GameplayStatics.BreakHitResult` _outhit)) (`self.Sword Damage`))
          (`KismetSystemLibrary.Delay` 0.3)
          (goto _label :!via `Reset`))))))

(event `/Game/Blueprints/BPI_Damage.Death`
  (`CharacterMovementComponent.DisableMovement` (`self.CharacterMovement`))
  (`PrimitiveComponent.SetSimulatePhysics` (`self.Mesh`) true)
  (set `self.IsDead?` true))

(event `/Game/Blueprints/BPI_Damage.Point Damage Trace`
  (bind _returnvalue (`SceneComponent.K2_GetComponentLocation` (`self.Point Trace Pos`)))
  (bind (_outhit _returnvalue_2) (`KismetSystemLibrary.SphereTraceSingleForObjects` :`Start` _returnvalue :`End` _returnvalue :`Radius` (`self.Point Attack Radius`) :`ObjectTypes` (`|MakeArray` "ObjectTypeQuery3" :!type "EObjectTypeQuery Enum") :`DrawDebugType` "ForDuration" :`DrawTime` 1.0))
  (if _returnvalue_2
    (bind (_bblockinghit _binitialoverlap _time _distance _location _impactpoint _normal _impactnormal _physmat _hitactor) (`GameplayStatics.BreakHitResult` _outhit))
    (`GameplayStatics.ApplyDamage` _hitactor 15.0)
    (`KismetSystemLibrary.Delay` 0.3)
    (`GameplayStatics.PlayWorldCameraShake` "/Game/Blueprints/BP_CameraShake_Attack.BP_CameraShake_Attack_C" _location 0.0 2000.0)))

(fn `Big Attack`
  (returns (Duration :type "Float (double-precision)"))
  (bind _returnvalue (`self.PlayAnimMontage` (`self.Big Attack Montage`)))
  (`GameplayStatics.PlaySoundAtLocation` "/Game/Audio/Sounds/SC_GruxAttack.SC_GruxAttack" (`self.K2_GetActorLocation`) (struct) 1.0 1.0 0.0 null null null null)
  (return _returnvalue))

(fn `Sword Attack`
  (returns (Duration :type "Float (double-precision)"))
  (bind _returnvalue (`self.PlayAnimMontage` (`self.Sword Attack Montage`)))
  (`GameplayStatics.PlaySoundAtLocation` "/Game/Audio/Sounds/SC_GruxAttack.SC_GruxAttack" (`self.K2_GetActorLocation`) (struct) 1.0 1.0 0.0 null null null null)
  (return _returnvalue))

(fn `UserConstructionScript`)