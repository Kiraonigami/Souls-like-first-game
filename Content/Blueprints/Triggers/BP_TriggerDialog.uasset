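; BP_TriggerDialog is a trigger actor that shows a timed dialog box on screen.
; When its Box component is overlapped, it creates a WB_DialogBox widget, fills its Dialog text from TextToDisplay0 and adds it to the viewport.
; After a delay of Duration0, it removes the widget; the overlap has no actor filter or one-shot guard.
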(event `self.Box.OnComponentBeginOverlap`
  (params (OverlappedComponent :type "PrimitiveComponent Object Reference") (OtherActor :type "Actor Object Reference") (OtherComp :type "PrimitiveComponent Object Reference") (OtherBodyIndex :type Integer) (bFromSweep :type Boolean) (SweepResult :type "HitResult Structure (by ref)"))
  (bind _wb_dialog (`self.WB_dialog`))
  (bind _returnvalue (`|CreateWidget` "/Game/UI/WB_DialogBox.WB_DialogBox_C"))
  (bind _output_get (set `self.WB_dialog` _returnvalue))
  (set `TextBlock.Text` (`KismetTextLibrary.Conv_StringToText` (`self.Text To Display_0`)) (`/Game/UI/WB_DialogBox.Dialog` _wb_dialog))
  (`UserWidget.AddToViewport` _output_get 0)
  (`KismetSystemLibrary.Delay` (`self.Duration_0`))
  (`Widget.RemoveFromParent` _wb_dialog))

(fn `UserConstructionScript`)