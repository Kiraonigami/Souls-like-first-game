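; BPC_Stats is a stats component that tracks health and stamina for its owning actor.
; IncreaseValue adjusts the chosen stat, clamps it between zero and its maximum, and updates the matching progress bar supplied through setter events.
; A looping timer regenerates stamina while the RegainStamina flag is set.
; When a health change leaves it at zero, Death sends DeathMessage to the owner.
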(event `self.ReceiveBeginPlay`
  (`KismetSystemLibrary.K2_SetTimerDelegate` (delegate `Regain Stamina`) 0.1 true))

(event `Regain Stamina`
  (if (`self.Regain Stamina?`)
    (`self.Increase Value` "NewEnumerator1" 0.5)))

(event `Death`
  (message `/Game/Blueprints/BPI_Damage.Death` (`self.GetOwner`)))

(event `Set Health Progress Bar`
  (params (`Health Progress Bar` :type "ProgressBar Object Reference"))
  (set `self.Health Progress Bar` `Health Progress Bar`))

(event `Set Stamina Progress Bar`
  (params (`Stamina Progress Bar` :type "ProgressBar Object Reference"))
  (set `self.Stamina Progress Bar` `Stamina Progress Bar`))

(fn `Increase Value`
  (params (Stat :type "/Game/Blueprints/e_stats Enum" :default "NewEnumerator0") (Value :type "Float (double-precision)"))
  (switch `/Game/Blueprints/e_stats` Stat
    (:`NewEnumerator0`
      (set `self.Health` (`KismetMathLibrary.FClamp` (+ (`self.Health`) Value) 0.0 (`self.Max Health`)))
      (`|ExecutionSequence`
        (:`then_0`
          (if (<= (`self.Health`) 0.0)
            (`self.Death`)))
        (:`then_1`
          (bind _health_progress_bar (`self.Health Progress Bar`)
            (:`then`
              (`ProgressBar.SetPercent` _health_progress_bar (/ (`self.Health`) (`self.Max Health`))))
            (:`else`)))))
    (:`NewEnumerator1`
      (set `self.Stamina` (`KismetMathLibrary.FClamp` (+ (`self.Stamina`) Value) 0.0 (`self.Max Stamina`)))
      (bind _stamina_progress_bar (`self.Stamina Progress Bar`)
        (:`then`
          (`ProgressBar.SetPercent` _stamina_progress_bar (/ (`self.Stamina`) (`self.Max Stamina`))))
        (:`else`)))))